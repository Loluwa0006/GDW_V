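; Base Blueprint for interactable entities that tracks whether the player is within range.
; Actor begin and end overlaps filter for PlayerBP and call OnPlayerEnter and OnPlayerExit, which switch the Interactable flag on and off.
; OnObjectInteracted fires the ObjectInteractedWith event dispatcher, without checking the flag itself.
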(event `self.ReceiveActorEndOverlap`
  (params (OtherActor :type "Actor Object Reference"))
  (cast `/Game/Blueprints/Player/PlayerBP` OtherActor)
  (`self.OnPlayerExit`))

(event `self.ReceiveActorBeginOverlap`
  (params (OtherActor :type "Actor Object Reference"))
  (cast `/Game/Blueprints/Player/PlayerBP` OtherActor)
  (`self.OnPlayerEnter`))

(fn `OnObjectInteracted`
  (`self.ObjectInteractedWith`))

(fn `OnPlayerEnter`
  (set `self.Interactable` true))

(fn `OnPlayerExit`
  (set `self.Interactable` false))

(fn `UserConstructionScript`)